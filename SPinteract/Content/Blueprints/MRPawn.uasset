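; Mixed reality player pawn that spawns left and right UXT hand interaction actors and runs head, eye and hand tracking every tick.
; Head tracking line-traces along the HMD forward vector and triggers gaze interaction on any GazeCube it hits.
; Eye gaze tracking only traces and draws a debug line from the camera along the gaze direction.
; Hand tracking draws debug axes at every keypoint of both tracked hands.
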(event `self.ReceiveTick`
  (params (DeltaSeconds :type "Float (single-precision)"))
  (`self.HeadTracking`)
  (`self.GazeTracking`)
  (`self.TrackingHands`))

(event `self.ReceiveBeginPlay`
  (bind _returnvalue (`KismetMathLibrary.MakeTransform` (0.0 0.0 0.0)))
  ;[1 1 1] Spawn Hand
  (`|SpawnActorFromClass` "/Script/UXTools.UxtHandInteractionActor" _returnvalue "Undefined" "OverrideRootScale" self true "Left" null)
  (`|SpawnActorFromClass` "/Script/UXTools.UxtHandInteractionActor" _returnvalue "Undefined" "OverrideRootScale" self true "Right" null))

(event `GazeTracking`
  (bind _returnvalue (`SceneComponent.K2_GetComponentLocation` (`self.Camera`)))
  ;[1 1 1] Eye Gaze Tracking
  (if (`EyeTrackerFunctionLibrary.IsEyeTrackerConnected`)
    (bind (_outgazedata _returnvalue_2) (`EyeTrackerFunctionLibrary.GetGazeData`))
    (if _returnvalue_2
      (`KismetSystemLibrary.LineTraceSingle` :`Start` _returnvalue :`End` (+ (* (`.GazeDirection` (break `EyeTrackerGazeData` _outgazedata)) 300.0) _returnvalue) :`TraceChannel` "TraceTypeQuery1" :`DrawDebugType` "ForOneFrame"))))

(event `HeadTracking`
  ;[1 1 1] Head Orientation Tracking
  (bind _hmddata (`HeadMountedDisplayFunctionLibrary.GetHMDData` self))
  (if (break `XRHMDData` _hmddata)
    (bind _output_get (set `self.HMDData Position` (`.Position` (break `XRHMDData` _hmddata))))
    (bind _outhit (`KismetSystemLibrary.LineTraceSingle` _output_get (+ (* (`KismetMathLibrary.GetForwardVector` (`KismetMathLibrary.Quat_Rotator` (`.Rotation` (break `XRHMDData` _hmddata)))) 500.0) (`self.HMDData Position`)) "TraceTypeQuery1"))
    (bind (_bblockinghit _binitialoverlap _time _distance _location _impactpoint _normal _impactnormal _physmat _hitactor _hitcomponent) (`GameplayStatics.BreakHitResult` _outhit))
    ;[1 1 1] Cast to Gaze Interaction
    (if _bblockinghit
      (bind _asgaze_cube (cast `/Game/Blueprints/GazeCube` _hitactor))
      (`/Game/Blueprints/GazeCube.InteractGaze` _asgaze_cube _hitcomponent))))

(event `TrackingHands`
  ;[1 1 1] Tracking Hands
  (for _index (range 2)
    (bind _motioncontrollerdata (`HeadMountedDisplayFunctionLibrary.GetMotionControllerData` null (select `int` _index :`0` "Left" :`1` "Right" :!type "EControllerHand Enum")))
    (bind (_bvalid _devicename _applicationinstanceid _devicevisualtype _handindex _trackingstatus _gripposition _griprotation _aimposition _aimrotation _handkeypositions _handkeyrotations) (break `XRMotionControllerData` _motioncontrollerdata))
    (if (and _bvalid (`|EnumEquality` _devicevisualtype "Hand"))
      (bind _enumvalue (foreach `EHandKeypoint` true)
        (:`LoopBody`
          (bind _returnvalue (`KismetMathLibrary.Conv_ByteToInt` _enumvalue))
          (`KismetSystemLibrary.DrawDebugCoordinateSystem` (`|GetArrayItem` _handkeypositions _returnvalue) (`KismetMathLibrary.Quat_Rotator` (`|GetArrayItem` _handkeyrotations _returnvalue)) 1.0 0.0 0.1))))))

(fn `UserConstructionScript`)